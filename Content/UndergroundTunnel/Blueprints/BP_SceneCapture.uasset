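; BP_SceneCapture is an actor with an orthographic 2D scene capture that publishes its capture bounds to materials in the underground tunnel project.
; It writes the capture's ortho width and the root's world location into the MPC_SceneCapture parameter collection as SceneCaptureSize and Position.
; The write runs in both the construction script and BeginPlay, with no per-tick update.
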(event EventBeginPlay
  (Rendering|Material|SetScalarParameterValue "/Game/UndergroundTunnel/Materials/MPC/MPC_SceneCapture.MPC_SceneCapture" "SceneCaptureSize" (Variables|/Script/Engine.SceneCaptureComponent2D|GetOrthoWidth (Variables|Default|GetSceneCaptureComponent2D)) :!class /Script/Engine.KismetMaterialLibrary)
  (Rendering|Material|SetVectorParameterValue "/Game/UndergroundTunnel/Materials/MPC/MPC_SceneCapture.MPC_SceneCapture" "Position" (Math|Conversions|ToLinearColor(Vector) (Transformation|GetWorldLocation (Variables|Default|GetDefaultSceneRoot))) :!class /Script/Engine.KismetMaterialLibrary))

(fn ConstructionScript
  (Rendering|Material|SetScalarParameterValue "/Game/UndergroundTunnel/Materials/MPC/MPC_SceneCapture.MPC_SceneCapture" "SceneCaptureSize" (Variables|/Script/Engine.SceneCaptureComponent2D|GetOrthoWidth (Variables|Default|GetSceneCaptureComponent2D)) :!class /Script/Engine.KismetMaterialLibrary)
  (Rendering|Material|SetVectorParameterValue "/Game/UndergroundTunnel/Materials/MPC/MPC_SceneCapture.MPC_SceneCapture" "Position" (Math|Conversions|ToLinearColor(Vector) (Transformation|GetWorldLocation (Variables|Default|GetDefaultSceneRoot))) :!class /Script/Engine.KismetMaterialLibrary))