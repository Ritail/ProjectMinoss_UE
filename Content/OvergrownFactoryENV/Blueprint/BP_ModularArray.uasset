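; Construction-script modular array tool that builds 3D grids of static mesh instances from the entries in AssetList.
; Each entry gets its own blocking HISM with optional material overrides, spaced by mesh bounds plus offset.
; A seeded stream jitters each instance's location, rotation and scale, though roll's upper bound is fixed at zero.
; Per-index edits then offset location and rotation, replace scale, or remove instances.
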(fn ConstructionScript
  (bind _stream (Variables|Default|GetStream))
  (bind _values (Utilities|Map|Values (Variables|Default|GetAssetList)))
  (for _array_element _values
    (bind _output_get (Variables|Default|SetCurrent%20Data _array_element))
    (Math|Random|SetRandomStreamSeed (Variables|Default|GetStream) (.seed _output_get))
    (bind _returnvalue (AddComponent|AddHierarchicalInstancedStaticMeshComponent false (.transform _output_get)))
    (bind _output_get_2 (Variables|Default|SetCurrentMesh_HISM _returnvalue))
    (Collision|SetCollisionProfileName _output_get_2 "BlockAll" true :!class /Script/Engine.PrimitiveComponent)
    (Components|StaticMesh|SetStaticMesh _output_get_2 (.mesh (Variables|Default|GetCurrent%20Data)))
    (if (.enbalematerialoverrides (Variables|Default|GetCurrent%20Data))
      (for (_array_element_2 _array_index) (.materialoverrides (Variables|Default|GetCurrent%20Data))
        (Rendering|Material|SetMaterial _returnvalue _array_index _array_element_2)
        (for _index (range 0 (- (.X (Utilities|Struct|BreakIntVector (.count (Variables|Default|GetCurrent%20Data)))) 1))
          (for _index_2 (range 0 (- (.Y (Utilities|Struct|BreakIntVector (.count (Variables|Default|GetCurrent%20Data)))) 1))
            (for _index_3 (range 0 (- (.Z (Utilities|Struct|BreakIntVector (.count (Variables|Default|GetCurrent%20Data)))) 1))
              (Components|InstancedStaticMesh|AddInstance (Variables|Default|GetCurrentMesh_HISM) (Math|Transform|MakeTransform (+ (Math|Vector|MakeVector (* _index (+ (.x (- (.max (StaticMesh|GetBoundingBox (.mesh (Variables|Default|GetCurrent%20Data)))) (.min (StaticMesh|GetBoundingBox (.mesh (Variables|Default|GetCurrent%20Data)))))) (.X (Math|Vector|BreakVector (.offset (Variables|Default|GetCurrent%20Data)))))) (* _index_2 (+ (.Y (Math|Vector|BreakVector (.offset (Variables|Default|GetCurrent%20Data)))) (.y (- (.max (StaticMesh|GetBoundingBox (.mesh (Variables|Default|GetCurrent%20Data)))) (.min (StaticMesh|GetBoundingBox (.mesh (Variables|Default|GetCurrent%20Data)))))))) (* _index_3 (+ (.Z (Math|Vector|BreakVector (.offset (Variables|Default|GetCurrent%20Data)))) (.z (- (.max (StaticMesh|GetBoundingBox (.mesh (Variables|Default|GetCurrent%20Data)))) (.min (StaticMesh|GetBoundingBox (.mesh (Variables|Default|GetCurrent%20Data))))))))) (Math|Vector|MakeVector (Math|Random|RandomFloatinRangefromStream (.x (.Location (Math|Transform|BreakTransform (.transformmin (Variables|Default|GetCurrent%20Data))))) (.x (.Location (Math|Transform|BreakTransform (.transformmax (Variables|Default|GetCurrent%20Data))))) _stream) (Math|Random|RandomFloatinRangefromStream (.y (.Location (Math|Transform|BreakTransform (.transformmin (Variables|Default|GetCurrent%20Data))))) (.y (.Location (Math|Transform|BreakTransform (.transformmax (Variables|Default|GetCurrent%20Data))))) _stream) (Math|Random|RandomFloatinRangefromStream (.z (.Location (Math|Transform|BreakTransform (.transformmin (Variables|Default|GetCurrent%20Data))))) (.z (.Location (Math|Transform|BreakTransform (.transformmax (Variables|Default|GetCurrent%20Data))))) _stream))) (Math|Rotator|MakeRotator (Math|Random|RandomFloatinRangefromStream (.roll (.Rotation (Math|Transform|BreakTransform (.transformmin (Variables|Default|GetCurrent%20Data))))) 0.0 _stream) (Math|Random|RandomFloatinRangefromStream (.pitch (.Rotation (Math|Transform|BreakTransform (.transformmin (Variables|Default|GetCurrent%20Data))))) (.pitch (.Rotation (Math|Transform|BreakTransform (.transformmax (Variables|Default|GetCurrent%20Data))))) _stream) (Math|Random|RandomFloatinRangefromStream (.yaw (.Rotation (Math|Transform|BreakTransform (.transformmin (Variables|Default|GetCurrent%20Data))))) (.yaw (.Rotation (Math|Transform|BreakTransform (.transformmax (Variables|Default|GetCurrent%20Data))))) _stream)) (Math|Vector|MakeVector (Math|Random|RandomFloatinRangefromStream (.x (.Scale (Math|Transform|BreakTransform (.transformmin (Variables|Default|GetCurrent%20Data))))) (.x (.Scale (Math|Transform|BreakTransform (.transformmax (Variables|Default|GetCurrent%20Data))))) _stream) (Math|Random|RandomFloatinRangefromStream (.y (.Scale (Math|Transform|BreakTransform (.transformmin (Variables|Default|GetCurrent%20Data))))) (.y (.Scale (Math|Transform|BreakTransform (.transformmax (Variables|Default|GetCurrent%20Data))))) _stream) (Math|Random|RandomFloatinRangefromStream (.z (.Scale (Math|Transform|BreakTransform (.transformmin (Variables|Default|GetCurrent%20Data))))) (.z (.Scale (Math|Transform|BreakTransform (.transformmax (Variables|Default|GetCurrent%20Data))))) _stream))) false)
              (if (.enbalematerialoverrides (Variables|Default|GetCurrent%20Data))
                (for (_array_element_3 _array_index_2) (.materialoverrides (Variables|Default|GetCurrent%20Data))
                  (Rendering|Material|SetMaterial _returnvalue _array_index_2 _array_element_3))))))
        (for _array_element_4 (.instancetransform (Variables|Default|GetCurrent%20Data))
          (Components|InstancedStaticMesh|UpdateInstanceTransform (Variables|Default|GetCurrentMesh_HISM) (.ID (Utilities|Struct|BreakF_InstanceData _array_element_4)) (Math|Transform|MakeTransform (+ (.location (.OutInstanceTransform (Components|InstancedStaticMesh|GetInstanceTransform (Variables|Default|GetCurrentMesh_HISM) (.ID (Utilities|Struct|BreakF_InstanceData _array_element_4)) false))) (.location (.Transform (Utilities|Struct|BreakF_InstanceData _array_element_4)))) (Math|Rotator|MakeRotator (+ (.roll (.rotation (.OutInstanceTransform (Components|InstancedStaticMesh|GetInstanceTransform (Variables|Default|GetCurrentMesh_HISM) (.ID (Utilities|Struct|BreakF_InstanceData _array_element_4)) false)))) (.roll (.rotation (.Transform (Utilities|Struct|BreakF_InstanceData _array_element_4))))) (+ (.pitch (.rotation (.OutInstanceTransform (Components|InstancedStaticMesh|GetInstanceTransform (Variables|Default|GetCurrentMesh_HISM) (.ID (Utilities|Struct|BreakF_InstanceData _array_element_4)) false)))) (.pitch (.rotation (.Transform (Utilities|Struct|BreakF_InstanceData _array_element_4))))) (+ (.yaw (.rotation (.OutInstanceTransform (Components|InstancedStaticMesh|GetInstanceTransform (Variables|Default|GetCurrentMesh_HISM) (.ID (Utilities|Struct|BreakF_InstanceData _array_element_4)) false)))) (.yaw (.rotation (.Transform (Utilities|Struct|BreakF_InstanceData _array_element_4)))))) (.scale (.Transform (Utilities|Struct|BreakF_InstanceData _array_element_4)))) false false false))
        (for _array_element_5 (.removeinstance (Variables|Default|GetCurrent%20Data))
          (Class|InstancedStaticMeshComponent|RemoveInstance (Variables|Default|GetCurrentMesh_HISM) _array_element_5)))
      (else
        (for _index_4 (range 0 (- (.X (Utilities|Struct|BreakIntVector (.count (Variables|Default|GetCurrent%20Data)))) 1))
          (for _index_5 (range 0 (- (.Y (Utilities|Struct|BreakIntVector (.count (Variables|Default|GetCurrent%20Data)))) 1))
            (for _index_6 (range 0 (- (.Z (Utilities|Struct|BreakIntVector (.count (Variables|Default|GetCurrent%20Data)))) 1))
              (Components|InstancedStaticMesh|AddInstance (Variables|Default|GetCurrentMesh_HISM) (Math|Transform|MakeTransform (+ (Math|Vector|MakeVector (* _index_4 (+ (.x (- (.max (StaticMesh|GetBoundingBox (.mesh (Variables|Default|GetCurrent%20Data)))) (.min (StaticMesh|GetBoundingBox (.mesh (Variables|Default|GetCurrent%20Data)))))) (.X (Math|Vector|BreakVector (.offset (Variables|Default|GetCurrent%20Data)))))) (* _index_5 (+ (.Y (Math|Vector|BreakVector (.offset (Variables|Default|GetCurrent%20Data)))) (.y (- (.max (StaticMesh|GetBoundingBox (.mesh (Variables|Default|GetCurrent%20Data)))) (.min (StaticMesh|GetBoundingBox (.mesh (Variables|Default|GetCurrent%20Data)))))))) (* _index_6 (+ (.Z (Math|Vector|BreakVector (.offset (Variables|Default|GetCurrent%20Data)))) (.z (- (.max (StaticMesh|GetBoundingBox (.mesh (Variables|Default|GetCurrent%20Data)))) (.min (StaticMesh|GetBoundingBox (.mesh (Variables|Default|GetCurrent%20Data))))))))) (Math|Vector|MakeVector (Math|Random|RandomFloatinRangefromStream (.x (.Location (Math|Transform|BreakTransform (.transformmin (Variables|Default|GetCurrent%20Data))))) (.x (.Location (Math|Transform|BreakTransform (.transformmax (Variables|Default|GetCurrent%20Data))))) _stream) (Math|Random|RandomFloatinRangefromStream (.y (.Location (Math|Transform|BreakTransform (.transformmin (Variables|Default|GetCurrent%20Data))))) (.y (.Location (Math|Transform|BreakTransform (.transformmax (Variables|Default|GetCurrent%20Data))))) _stream) (Math|Random|RandomFloatinRangefromStream (.z (.Location (Math|Transform|BreakTransform (.transformmin (Variables|Default|GetCurrent%20Data))))) (.z (.Location (Math|Transform|BreakTransform (.transformmax (Variables|Default|GetCurrent%20Data))))) _stream))) (Math|Rotator|MakeRotator (Math|Random|RandomFloatinRangefromStream (.roll (.Rotation (Math|Transform|BreakTransform (.transformmin (Variables|Default|GetCurrent%20Data))))) 0.0 _stream) (Math|Random|RandomFloatinRangefromStream (.pitch (.Rotation (Math|Transform|BreakTransform (.transformmin (Variables|Default|GetCurrent%20Data))))) (.pitch (.Rotation (Math|Transform|BreakTransform (.transformmax (Variables|Default|GetCurrent%20Data))))) _stream) (Math|Random|RandomFloatinRangefromStream (.yaw (.Rotation (Math|Transform|BreakTransform (.transformmin (Variables|Default|GetCurrent%20Data))))) (.yaw (.Rotation (Math|Transform|BreakTransform (.transformmax (Variables|Default|GetCurrent%20Data))))) _stream)) (Math|Vector|MakeVector (Math|Random|RandomFloatinRangefromStream (.x (.Scale (Math|Transform|BreakTransform (.transformmin (Variables|Default|GetCurrent%20Data))))) (.x (.Scale (Math|Transform|BreakTransform (.transformmax (Variables|Default|GetCurrent%20Data))))) _stream) (Math|Random|RandomFloatinRangefromStream (.y (.Scale (Math|Transform|BreakTransform (.transformmin (Variables|Default|GetCurrent%20Data))))) (.y (.Scale (Math|Transform|BreakTransform (.transformmax (Variables|Default|GetCurrent%20Data))))) _stream) (Math|Random|RandomFloatinRangefromStream (.z (.Scale (Math|Transform|BreakTransform (.transformmin (Variables|Default|GetCurrent%20Data))))) (.z (.Scale (Math|Transform|BreakTransform (.transformmax (Variables|Default|GetCurrent%20Data))))) _stream))) false)
              (if (.enbalematerialoverrides (Variables|Default|GetCurrent%20Data))
                (for (_array_element_6 _array_index_3) (.materialoverrides (Variables|Default|GetCurrent%20Data))
                  (Rendering|Material|SetMaterial _returnvalue _array_index_3 _array_element_6))))))
        (for _array_element_7 (.instancetransform (Variables|Default|GetCurrent%20Data))
          (Components|InstancedStaticMesh|UpdateInstanceTransform (Variables|Default|GetCurrentMesh_HISM) (.ID (Utilities|Struct|BreakF_InstanceData _array_element_7)) (Math|Transform|MakeTransform (+ (.location (.OutInstanceTransform (Components|InstancedStaticMesh|GetInstanceTransform (Variables|Default|GetCurrentMesh_HISM) (.ID (Utilities|Struct|BreakF_InstanceData _array_element_7)) false))) (.location (.Transform (Utilities|Struct|BreakF_InstanceData _array_element_7)))) (Math|Rotator|MakeRotator (+ (.roll (.rotation (.OutInstanceTransform (Components|InstancedStaticMesh|GetInstanceTransform (Variables|Default|GetCurrentMesh_HISM) (.ID (Utilities|Struct|BreakF_InstanceData _array_element_7)) false)))) (.roll (.rotation (.Transform (Utilities|Struct|BreakF_InstanceData _array_element_7))))) (+ (.pitch (.rotation (.OutInstanceTransform (Components|InstancedStaticMesh|GetInstanceTransform (Variables|Default|GetCurrentMesh_HISM) (.ID (Utilities|Struct|BreakF_InstanceData _array_element_7)) false)))) (.pitch (.rotation (.Transform (Utilities|Struct|BreakF_InstanceData _array_element_7))))) (+ (.yaw (.rotation (.OutInstanceTransform (Components|InstancedStaticMesh|GetInstanceTransform (Variables|Default|GetCurrentMesh_HISM) (.ID (Utilities|Struct|BreakF_InstanceData _array_element_7)) false)))) (.yaw (.rotation (.Transform (Utilities|Struct|BreakF_InstanceData _array_element_7)))))) (.scale (.Transform (Utilities|Struct|BreakF_InstanceData _array_element_7)))) false false false))
        (for _array_element_8 (.removeinstance (Variables|Default|GetCurrent%20Data))
          (Class|InstancedStaticMeshComponent|RemoveInstance (Variables|Default|GetCurrentMesh_HISM) _array_element_8))))))